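; Gameplay ability that plays the character's SimpleAbilityMontage and applies a damage effect on a gameplay event.
; After committing, it plays the montage and waits for one Player.Ability.Simple event, whose target data receives GE_SimpleAbility_Damage.
; The ability ends after applying the effect or when the montage completes, blends out, is interrupted or is cancelled.
; OnEndAbility cleans up the montage and event-wait tasks.
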(event `self.K2_ActivateAbility`
  (bind _returnvalue_owneractor (break `GameplayAbilityActorInfo` (`self.GetActorInfo`)))
  (`KismetSystemLibrary.PrintString` "GA_SimpleAbility : Activated")
  (`self.K2_CommitAbility`)
  (bind _aseacharacter (cast `EACharacter` _returnvalue_owneractor))
  (bind _asynctaskproxy (`AbilityTask_PlayMontageAndWait.CreatePlayMontageAndWaitProxy` "None" (`EACharacter.SimpleAbilityMontage` _aseacharacter))
    (:`then`
      (set `self.Async Task` _asynctaskproxy)
      (`KismetSystemLibrary.PrintString` "GA_SimpleAbility : Waiting for event")
      (bind (_asynctaskproxy_2 _payload) (`AbilityTask_WaitGameplayEvent.WaitGameplayEvent` (struct :`TagName` "Player.Ability.Simple") null true)
        (:`then`
          (set `self.Async Task_0` _asynctaskproxy_2))
        (:`EventReceived`
          (`KismetSystemLibrary.PrintString` "GA_SimpleAbility :  Recieved")
          (`self.BP_ApplyGameplayEffectToTarget` (`.TargetData` (break `GameplayEventData` _payload)) "/Game/Blueprints/Abilities/SimpleAbility/GE_SimpleAbility_Damage.GE_SimpleAbility_Damage_C")
          (`self.K2_EndAbility`))))
    (:`OnCompleted`
      (`self.K2_EndAbility` :!label _label))
    (:`OnBlendOut`
      (goto _label))
    (:`OnInterrupted`
      (goto _label))
    (:`OnCancelled`
      (goto _label))))

(event `self.K2_OnEndAbility`
  (params (bWasCancelled :type Boolean))
  (bind _async_task (`self.Async Task`))
  (bind _async_task_0 (`self.Async Task_0`))
  (`/Engine/EditorBlueprintResources/StandardMacros.IsValid` _async_task
    (:`Is Valid`
      (`GameplayTask.EndTask` _async_task)
      (`/Engine/EditorBlueprintResources/StandardMacros.IsValid` _async_task_0
        (:`Is Valid`
          (`GameplayTask.EndTask` _async_task_0))))))