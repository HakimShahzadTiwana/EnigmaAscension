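; GA_Block is a Gameplay Ability that makes an EACharacter block.
; On activation it applies GE_Block to the owner, commits the ability, then plays the character's BlockAbilityMontage.
; Completion, blend-out, interruption or cancellation of the montage ends the ability, with debug prints marking start and end.
; The live path never removes GE_Block; unconnected leftover nodes hold toggle-stop, effect removal and Abilities.Block tag checks.
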(event `self.K2_ActivateAbility`
  (bind _returnvalue_owneractor (break `GameplayAbilityActorInfo` (`self.GetActorInfo`)))
  (`self.BP_ApplyGameplayEffectToOwner` "/Game/Blueprints/Abilities/Block/GE_Block.GE_Block_C")
  (`self.K2_CommitAbility`)
  (bind _aseacharacter (cast `EACharacter` _returnvalue_owneractor))
  (`AbilityTask_PlayMontageAndWait.CreatePlayMontageAndWaitProxy` "None" (`EACharacter.BlockAbilityMontage` _aseacharacter)
    (:`then`
      (`KismetSystemLibrary.PrintString` "Start Blocking"))
    (:`OnCompleted`
      (`self.K2_EndAbility` :!label _label)
      (`KismetSystemLibrary.PrintString` "End Blocking"))
    (:`OnBlendOut`
      (goto _label))
    (:`OnInterrupted`
      (goto _label))
    (:`OnCancelled`
      (goto _label))))