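; Gameplay ability for the primary attack: plays the character's attack montage and applies damage on the hit event unless the target is blocking.
; Clients and server player index 0 forward timestamp-free input records to the server through the player controller before attacking.
; For other players, the server offsets the montage start by their ping when rollback is enabled, compensating for latency.
; Non-server instances end on the hit event, otherwise on montage end.
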(event `self.K2_ActivateAbility`
  (bind (_returnvalue_owneractor _returnvalue_avataractor _returnvalue_playercontroller) (break `GameplayAbilityActorInfo` (`self.GetActorInfo`)))
  (`KismetSystemLibrary.PrintString` "GA_PrimaryAttack: Activated")
  (bind _aseaplayer_controller (cast `EAPlayerController` _returnvalue_playercontroller)
    (:`then`
      (bind _output_get (set `self.As EAPlayer Controller` _aseaplayer_controller))
      (bind _aseaplayer_state (cast `EAPlayerState` (`Controller.PlayerState` _output_get))
        (:`then`
          (set `self.As EAPlayer State` _aseaplayer_state)
          (bind _aseacharacter (cast `EACharacter` _returnvalue_owneractor)
            (:`then`
              (set `self.As EACharacter` _aseacharacter)
              (`self.K2_CommitAbility`)
              (if (`KismetSystemLibrary.IsServer`)
                (if (== (`EAPlayerState.GetPlayerIndex` (`self.As EAPlayer State`)) 0)
                  (`self.ForwardClientInputs`)
                  (else
                    (bind _asbp_eagame_instance (cast `/Game/Blueprints/Core/BP_EAGameInstance` (`GameplayStatics.GetGameInstance`)))
                    (if (`EAGameInstance.bIsRollbackSet` _asbp_eagame_instance)
                      (set `self.MontageSkip` (`PlayerState.GetPingInMilliseconds` (`self.As EAPlayer State`))))
                    (`self.Start Attack`)))
                (else
                  (`self.ForwardClientInputs`))))
            (:`CastFailed`
              (`KismetSystemLibrary.PrintString` "Player Character Cast Failed")
              (`self.K2_EndAbility`))))
        (:`CastFailed`
          (`KismetSystemLibrary.PrintString` "Player State Cast Failed")
          (`self.K2_EndAbility`))))
    (:`CastFailed`
      (`KismetSystemLibrary.PrintString` "Player Controller Cast Failed")
      (`self.K2_EndAbility`))))

(event `ForwardClientInputs`
  (bind _returnvalue (`EAPlayerController.Client_CollectInputData` (`self.As EAPlayer Controller`) "PrimaryAttack" (0.0 0.0 0.0) -1))
  (`EAPlayerController.Server_CollectInputData` (`self.As EAPlayer Controller`) _returnvalue)
  (set `EACharacter.CurrentInputID` (`.PlayerInputID` (break `PlayerInputData` _returnvalue)) (`self.As EACharacter`))
  (`self.Start Attack`))

(event `Start Attack`
  (`KismetSystemLibrary.PrintString` (`KismetStringLibrary.Concat_StrStr` "Plsying Montage with miliseconds skipped : " (`KismetStringLibrary.Conv_DoubleToString` (`self.MontageSkip`))) true true (struct :`R` 1.0 :`B` 0.355044 :`A` 1.0))
  (bind _asynctaskproxy (`AbilityTask_PlayMontageAndWait.CreatePlayMontageAndWaitProxy` "None" (`EACharacter.PrimaryAttackMontage` (`self.As EACharacter`)) 1.0 "None" true 1.0 (/ (`self.MontageSkip`) 1000.0))
    (:`then`
      (set `self.Async Task_0` _asynctaskproxy)
      (`KismetSystemLibrary.PrintString` "GA_PrimaryAttack: Waiting for event")
      (bind (_asynctaskproxy_2 _payload) (`AbilityTask_WaitGameplayEvent.WaitGameplayEvent` (struct :`TagName` "Player.Attack.Primary") null true)
        (:`then`
          (set `self.Async Task` _asynctaskproxy_2))
        (:`EventReceived`
          (`KismetSystemLibrary.PrintString` "GA_PrimaryAttack : Recieved")
          (bind (_eventtag _instigator _target _optionalobject _optionalobject2 _contexthandle _instigatortags _targettags _eventmagnitude _targetdata) (break `GameplayEventData` _payload))
          (if (`BlueprintGameplayTagLibrary.HasTag` _targettags (struct :`TagName` "Abilities.Block"))
            (`KismetSystemLibrary.PrintString` "Target Actor Is Blocking GE_Primary_Attack_Damage NOT Applied")
            (else
              (`KismetSystemLibrary.PrintString` "Target Actor Is NOT Blocking GE_Primary_Attack_Damage Applied")
              (`self.BP_ApplyGameplayEffectToTarget` _targetdata "/Game/Blueprints/Abilities/PrimaryAttack/GE_PrimaryAttack_Damage.GE_PrimaryAttack_Damage_C")))
          (if (not (`KismetSystemLibrary.IsServer`))
            (`KismetSystemLibrary.PrintString` "Calling for client GA_Primary Attack " true true (struct :`G` 0.66 :`B` 1.0 :`A` 1.0) 300.0)
            (`self.K2_EndAbility`)))))
    (:`OnCompleted`
      (`self.K2_EndAbility` :!label _label))
    (:`OnBlendOut`
      (goto _label))
    (:`OnInterrupted`
      (goto _label))
    (:`OnCancelled`
      (goto _label))))

(event `self.K2_OnEndAbility`
  (params (bWasCancelled :type Boolean))
  (bind _async_task (`self.Async Task`))
  (bind _async_task_0 (`self.Async Task_0`))
  (`/Engine/EditorBlueprintResources/StandardMacros.IsValid` _async_task
    (:`Is Valid`
      (`GameplayTask.EndTask` _async_task)
      (`/Engine/EditorBlueprintResources/StandardMacros.IsValid` _async_task_0
        (:`Is Valid`
          (`GameplayTask.EndTask` _async_task_0))))))