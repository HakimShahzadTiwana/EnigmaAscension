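; GA_Sprint is a gameplay ability that lets an EACharacter sprint while its input is held.
; On activation it caches the character's max walk speed, raises it by half and waits for input release to end the ability.
; When the ability ends it restores the cached speed on the movement component, and debug prints report activation, release and cast failure.
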(event `self.K2_ActivateAbility`
  (bind _returnvalue_owneractor (break `GameplayAbilityActorInfo` (`self.GetActorInfo`)))
  (`KismetSystemLibrary.PrintString` "Sprint Activated")
  (bind _aseacharacter (cast `EACharacter` _returnvalue_owneractor)
    (:`then`
      (bind _charactermovement (`Character.CharacterMovement` _aseacharacter))
      (bind _output_get (set `self.DefaultMaxWalkSpeed` (`CharacterMovementComponent.MaxWalkSpeed` _charactermovement)))
      (set `CharacterMovementComponent.MaxWalkSpeed` (* _output_get 1.5) _charactermovement)
      (`AbilityTask_WaitInputRelease.WaitInputRelease` true
        (:`OnRelease`
          (`KismetSystemLibrary.PrintString` "Sprint Deactivated")
          (`self.K2_EndAbility`))))
    (:`CastFailed`
      (`KismetSystemLibrary.PrintString` "Cast Failed"))))

(event `self.K2_OnEndAbility`
  (params (bWasCancelled :type Boolean))
  (bind _returnvalue_owneractor (break `GameplayAbilityActorInfo` (`self.GetActorInfo`)))
  (bind _aseacharacter (cast `EACharacter` _returnvalue_owneractor))
  (set `CharacterMovementComponent.MaxWalkSpeed` (`self.DefaultMaxWalkSpeed`) (`Character.CharacterMovement` _aseacharacter)))