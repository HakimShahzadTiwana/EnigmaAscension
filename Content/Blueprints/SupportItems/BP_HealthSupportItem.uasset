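; BP_HealthSupportItem is a health support item that the player can interact with by pressing E while nearby.
; It enables input for the first player controller on BeginPlay so the actor receives the key press directly.
; On E, it queries SphereComponent for overlapping EACharacter actors and passes the first, cast to Pawn, to Interact.
; The Interact logic, including any health effect, is not defined in this graph.
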(event `self.ReceiveBeginPlay`
  (`self.EnableInput` (`GameplayStatics.GetPlayerController` 0)))

(event `Key|E`
  (params (Key :type "Key Structure"))
  (bind _overlappingactors (`PrimitiveComponent.GetOverlappingActors` (`self.SphereComponent`) "/Script/EnigmaAscension.EACharacter"))
  (:`Pressed`
    (if (> (`KismetArrayLibrary.Array_Length` _overlappingactors) 0)
      (bind _aspawn (cast `Pawn` (`|GetArrayItem` _overlappingactors)))
      (`EAGameplayInterface.Interact` _aspawn))))

(fn `UserConstructionScript`)