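; Game instance that hosts, finds and joins multiplayer sessions through Advanced Sessions nodes, server-traveling to TestMap as listen server after creation.
; Custom session properties tag games for search filtering and carry creation time and public access.
; Results are cached raw and converted to SessionData, which sort, filter and search events replace before broadcasting OnSessionResultsFound.
; FindSteamSessionResult maps SessionData back to a raw result by server name.
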(event `self.CreateSession`
  (params (isPublic :type Boolean))
  ;[1 1 1] Session Logic
  (`KismetSystemLibrary.PrintString` "Core: GameInstance - Creating Sessions" true true (struct :`G` 1.0 :`A` 1.0))
  (`CreateSessionCallbackProxyAdvanced.CreateAdvancedSession` (`|MakeArray` (`AdvancedSessionsLibrary.MakeLiteralSessionPropertyString` "EA_Session_Type" "EA_Simple_Session") (`AdvancedSessionsLibrary.MakeLiteralSessionPropertyString` "CreationTime" (`self.GetDateTime`)) (`AdvancedSessionsLibrary.MakeLiteralSessionPropertyBool` "AccessType" isPublic)) (`GameplayStatics.GetPlayerController` 0) 8
    (:`OnSuccess`
      (`KismetSystemLibrary.PrintString` "Core: GameInstance -Created Session Successfully" true true (struct :`G` 1.0 :`A` 1.0))
      (`AdvancedSessionsLibrary.ServerTravel` "/Game/Maps/TestMap?listen"))
    (:`OnFailure`
      (`KismetSystemLibrary.PrintString` "Core: GameInstance -Create SessionFailed" true true (struct :`G` 1.0 :`A` 1.0)))))

(event `self.FindSessions`
  ;[1 1 1] Session Logic
  (`KismetSystemLibrary.PrintString` "Core: GameInstance - Finding Sessions" true true (struct :`G` 1.0 :`A` 1.0))
  (bind _results (`FindSessionsCallbackProxyAdvanced.FindSessionsAdvanced` (`GameplayStatics.GetPlayerController` 0) 10000 false "ClientServersOnly" (`|MakeArray` (`AdvancedSessionsLibrary.MakeLiteralSessionSearchProperty` (`AdvancedSessionsLibrary.MakeLiteralSessionPropertyString` "EA_Session_Type" "EA_Simple_Session") "Equals")))
    (:`then`
      (`KismetSystemLibrary.PrintString` (`KismetStringLibrary.Concat_StrStr` "Core: GameInstance -Number of Sessions found Successfully : " (`KismetStringLibrary.Conv_IntToString` (`KismetArrayLibrary.Array_Length` _results))) true true (struct :`G` 1.0 :`A` 1.0))
      (`self.SaveSteamSessionsData` _results)
      (`self.On Session Results Found`))
    (:`OnFailure`
      (`KismetSystemLibrary.PrintString` "Core : Game Instance - Find Session Failed" true true (struct :`G` 1.0 :`A` 1.0)))))

(event `Join Selected Session`
  (params (SearchResult :type "BlueprintSessionResult Structure (by ref)"))
  ;[1 1 1] Session Logic
  (`KismetSystemLibrary.PrintString` (`KismetStringLibrary.Concat_StrStr` "Core: Game instance - Join selected session : " (`FindSessionsCallbackProxy.GetServerName` SearchResult)) true true (struct :`G` 1.0 :`A` 1.0))
  (`JoinSessionCallbackProxy.JoinSession` (`GameplayStatics.GetPlayerController` 0) SearchResult
    (:`OnSuccess`
      (`KismetSystemLibrary.PrintString` "Core: Game Instace - Join Session Succeded" true true (struct :`G` 1.0 :`A` 1.0)))
    (:`OnFailure`
      (`KismetSystemLibrary.PrintString` "Core: Game Instace - Join Session Failed" true true (struct :`G` 1.0 :`A` 1.0)))))

(event `Sort Sessions`
  ;[1 1 1] Session Logic
  (bind _returnvalue (`self.SortSessionData`))
  (set `self.SessionData` _returnvalue)
  (`self.On Session Results Found`))

(event `Filter Sessions`
  (params (publicMatch :type Boolean) (Hostname :type String))
  ;[1 1 1] Session Logic
  (bind _returnvalue (`self.FilterSessionData` publicMatch Hostname))
  (set `self.SessionData` _returnvalue)
  (`self.On Session Results Found`))

(event `Search Sessions`
  (params (UserQuery :type String))
  ;[1 1 1] Session Logic
  (bind _returnvalue (`self.SearchSessionData` UserQuery))
  (set `self.SessionData` _returnvalue)
  (`self.On Session Results Found`))

(fn `FindSteamSessionResult`
  (params (SessionData :type "SessionData Structure"))
  (returns (`Array Element` :type "BlueprintSessionResult Structure"))
  (for _array_element (`self.BlueprintSessionData`)
    (if (`KismetStringLibrary.EqualEqual_StrStr` (`FindSessionsCallbackProxy.GetServerName` _array_element) (`.Name` (break `SessionData` SessionData)))
      (return _array_element)))
  (return))

(fn `SaveSteamSessionsData`
  (params (Sessions :type "Array of BlueprintSessionResult Structure"))
  (set `self.BlueprintSessionData` Sessions)
  (`KismetArrayLibrary.Array_Clear` (`self.SessionData`))
  (for _array_element Sessions
    (bind _extrasettings (`AdvancedSessionsLibrary.GetExtraSettings` _array_element))
    (bind _settingvalue (`AdvancedSessionsLibrary.GetSessionPropertyString` _extrasettings "CreationTime")
      (:`Found`
        _)
      (:`NotFound`
        _))
    (bind _settingvalue_2 (`AdvancedSessionsLibrary.GetSessionPropertyBool` _extrasettings "AccessType")
      (:`Found`
        (`KismetArrayLibrary.Array_Add` (`self.SessionData`) (make `SessionData` (`FindSessionsCallbackProxy.GetServerName` _array_element) (`FindSessionsCallbackProxy.GetCurrentPlayers` _array_element) (`FindSessionsCallbackProxy.GetMaxPlayers` _array_element) _settingvalue _settingvalue_2)))))
  (`self.SaveSteamSessionsFound` (`self.SessionData`)))