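; BP_EAPlayerController is a player controller that handles character selection and requests spawns from BP_TestGameMode.
; On first possession it creates the WB_CharacterSelection widget, via ShowSelectionWidget on the server or directly otherwise, with a flag preventing repeats.
; Selection events, including a separate GreyStone path, forward to Server events that cast the game mode and pass this controller to its spawn functions.
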(event `Show Selection Widget`
  (bind _returnvalue (`|CreateWidget` "/Game/Blueprints/UI/InGame/WB_CharacterSelection.WB_CharacterSelection_C" :!label _label))
  (`UserWidget.AddToViewport` _returnvalue 0))

(event `self.ReceivePossess`
  (params (PossessedPawn :type "Pawn Object Reference"))
  (`KismetSystemLibrary.PrintString` (`KismetStringLibrary.Concat_StrStr` (`KismetSystemLibrary.GetDisplayName` PossessedPawn) "Has been possessed"))
  (if (`self.CharacterSelectionShown`)
    (`KismetSystemLibrary.PrintString` "Character has been selected")
    (else
      (set `self.CharacterSelectionShown` true)
      (if (`KismetSystemLibrary.IsServer`)
        (`self.Show Selection Widget`)
        (else
          (goto _label))))))

(event `CharacterSelected`
  (params (`Selected Character` :type "UEACharacters Enum" :default "Countess"))
  (`self.Server_CharacterSelected` `Selected Character`))

(event `Server_CharacterSelected`
  (params (`Selected Character` :type "UEACharacters Enum" :default "Countess"))
  (bind _asbp_test_game_mode (cast `/Game/Blueprints/Core/BP_TestGameMode` (`GameplayStatics.GetGameMode`)))
  (`/Game/Blueprints/Core/BP_TestGameMode.Spawn Character` _asbp_test_game_mode `Selected Character` self))

(event `GreyStoneSelected`
  (`self.Server_GreyStoneSelected`))

(event `Server_GreyStoneSelected`
  (bind _asbp_test_game_mode (cast `/Game/Blueprints/Core/BP_TestGameMode` (`GameplayStatics.GetGameMode`)))
  (`/Game/Blueprints/Core/BP_TestGameMode.Spawn GreyStone` _asbp_test_game_mode self))

(fn `UserConstructionScript`)